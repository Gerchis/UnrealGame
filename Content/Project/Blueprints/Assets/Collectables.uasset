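; Collectable pickup actor that increments the collectable count in ProjectInstance, the game instance, when the Player overlaps it.
; An Active flag limits it to one pickup, and the new total is printed as a string.
; The SizeCube timeline then animates the mesh's uniform scale while spinning it in yaw, and destroys the actor when finished.
; The construction script sizes the Cube box from the BoxSize variable.
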(event `self.ReceiveActorBeginOverlap`
  (params (OtherActor :type "Actor Object Reference"))
  (bind _asproject_instance (cast `/Game/Project/Blueprints/ProjectInstance` (`GameplayStatics.GetGameInstance`) :!pure true))
  (if (`self.Active`)
    (cast `/Game/Project/Blueprints/Character/Player` OtherActor)
    (set `/Game/Project/Blueprints/ProjectInstance.Collectable` (+ (`/Game/Project/Blueprints/ProjectInstance.Collectable` _asproject_instance) 1) _asproject_instance)
    (set `self.Active` false)
    (`self.EndEffect`)
    (`KismetSystemLibrary.PrintString` (`KismetStringLibrary.Conv_IntToString` (`/Game/Project/Blueprints/ProjectInstance.Collectable` (cast `/Game/Project/Blueprints/ProjectInstance` (`GameplayStatics.GetGameInstance`) :!pure true))))))

(event `EndEffect`
  (bind (_direction _newtrack_0) (`Timeline|SizeCube` :!via `PlayFromStart`)
    (:`Update`
      (`SceneComponent.SetWorldScale3D` (`self.StaticMesh`) (`KismetMathLibrary.MakeVector` _newtrack_0 _newtrack_0 _newtrack_0))
      (`SceneComponent.K2_AddLocalRotation` (`self.StaticMesh`) (`KismetMathLibrary.MakeRotator` 0.0 0.0 5.0) false false))
    (:`Finished`
      (`self.K2_DestroyActor`))))

(fn `UserConstructionScript`
  (`BoxComponent.SetBoxExtent` (`self.Cube`) (`self.BoxSize`) true))