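; Trigger volume between two areas that swaps the visible area as the player crosses its center on a chosen axis.
; Player overlap, while Active, enables Tick, which compares positions and gates each switch through CheckNewArea, whose area comparison is left unconnected.
; Switching hides the game instance's active actors, shows the new area's, records it and moves the camera.
; Construction sizes the collider and barrier from ColliderSize.
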(event `self.ReceiveTick`
  (params (DeltaSeconds :type "Float (single-precision)"))
  (bind (_returnvalue_x _returnvalue_y _returnvalue_z) (`KismetMathLibrary.BreakVector` (`self.K2_GetActorLocation`)))
  (bind (_returnvalue_x_2 _returnvalue_y_2) (`KismetMathLibrary.BreakVector` (`self.K2_GetActorLocation`)))
  (bind _returnvalue_x_3 (`KismetMathLibrary.BreakVector` (`self.K2_GetActorLocation`)))
  (bind (_returnvalue_x_4 _returnvalue_y_3) (`KismetMathLibrary.BreakVector` (`self.K2_GetActorLocation` (`GameplayStatics.GetPlayerPawn` 0))))
  (bind _returnvalue_x_5 (`KismetMathLibrary.BreakVector` (`self.K2_GetActorLocation` (`GameplayStatics.GetPlayerPawn` 0))))
  (bind (_returnvalue_x_6 _returnvalue_y_4 _returnvalue_z_2) (`KismetMathLibrary.BreakVector` (`self.K2_GetActorLocation` (`GameplayStatics.GetPlayerPawn` 0))))
  (switch `/Game/Project/Blueprints/VectorAxis` (`self.DirectionAxis`)
    (:`NewEnumerator0`
      (if (> _returnvalue_x_5 _returnvalue_x_3)
        (if (`self.CheckNewArea` (`self.SecondArea`))
          (`self.ChangeToSecond`))
        (elif (`self.CheckNewArea` (`self.FirstArea`))
          (`self.ChangeToFirst`))))
    (:`NewEnumerator1`
      (if (> _returnvalue_y_3 _returnvalue_y_2)
        (if (`self.CheckNewArea` (`self.SecondArea`))
          (`self.ChangeToSecond`))
        (elif (`self.CheckNewArea` (`self.FirstArea`))
          (`self.ChangeToFirst`))))
    (:`NewEnumerator2`
      (if (> _returnvalue_z_2 _returnvalue_z)
        (if (`self.CheckNewArea` (`self.SecondArea`))
          (`self.ChangeToSecond`))
        (elif (`self.CheckNewArea` (`self.FirstArea`))
          (`self.ChangeToFirst`))))))

(event `self.Collider.OnComponentBeginOverlap`
  (params (OverlappedComponent :type "PrimitiveComponent Object Reference") (OtherActor :type "Actor Object Reference") (OtherComp :type "PrimitiveComponent Object Reference") (OtherBodyIndex :type Integer) (bFromSweep :type Boolean) (SweepResult :type "HitResult Structure (by ref)"))
  (if (`self.Active`)
    (cast `/Game/Project/Blueprints/Character/Player` OtherActor)
    (`self.SetActorTickEnabled` true)))

(event `ChangeToFirst`
  (bind _asproject_instance (cast `/Game/Project/Blueprints/ProjectInstance` (`GameplayStatics.GetGameInstance`) :!pure true))
  (bind _activeareas (`/Game/Project/Blueprints/ProjectInstance.ActiveAreas` (cast `/Game/Project/Blueprints/ProjectInstance` (`GameplayStatics.GetGameInstance`) :!pure true)))
  (for _array_element _activeareas
    (`self.SetActorHiddenInGame` _array_element true))
  (`KismetArrayLibrary.Array_Clear` _activeareas)
  (for _array_element_2 (`/Game/Project/Blueprints/Triggers/AreaInfo.AreaActors` (`self.FirstArea`))
    (`self.SetActorHiddenInGame` _array_element_2 false)
    (`KismetArrayLibrary.Array_Add` (`/Game/Project/Blueprints/ProjectInstance.ActiveAreas` (cast `/Game/Project/Blueprints/ProjectInstance` (`GameplayStatics.GetGameInstance`) :!pure true)) _array_element_2))
  (set `/Game/Project/Blueprints/ProjectInstance.ActualArea` (`/Game/Project/Blueprints/Triggers/AreaInfo.SelfArea` (`self.FirstArea`)) _asproject_instance)
  (`/Game/Project/Blueprints/Character/Camera.MoveCamera` (`/Game/Project/Blueprints/ProjectInstance.GameCamera` _asproject_instance) (`/Game/Project/Blueprints/Triggers/AreaInfo.CameraPos` (`self.FirstArea`))))

(event `self.Collider.OnComponentEndOverlap`
  (params (OverlappedComponent :type "PrimitiveComponent Object Reference") (OtherActor :type "Actor Object Reference") (OtherComp :type "PrimitiveComponent Object Reference") (OtherBodyIndex :type Integer))
  (if (`self.Active`)
    (cast `/Game/Project/Blueprints/Character/Player` OtherActor)
    (`self.SetActorTickEnabled` false)))

(event `ChangeToSecond`
  (bind _asproject_instance (cast `/Game/Project/Blueprints/ProjectInstance` (`GameplayStatics.GetGameInstance`) :!pure true))
  (bind _activeareas (`/Game/Project/Blueprints/ProjectInstance.ActiveAreas` (cast `/Game/Project/Blueprints/ProjectInstance` (`GameplayStatics.GetGameInstance`) :!pure true)))
  (for _array_element _activeareas
    (`self.SetActorHiddenInGame` _array_element true))
  (`KismetArrayLibrary.Array_Clear` _activeareas)
  (for _array_element_2 (`/Game/Project/Blueprints/Triggers/AreaInfo.AreaActors` (`self.SecondArea`))
    (`self.SetActorHiddenInGame` _array_element_2 false)
    (`KismetArrayLibrary.Array_Add` (`/Game/Project/Blueprints/ProjectInstance.ActiveAreas` (cast `/Game/Project/Blueprints/ProjectInstance` (`GameplayStatics.GetGameInstance`) :!pure true)) _array_element_2))
  (set `/Game/Project/Blueprints/ProjectInstance.ActualArea` (`/Game/Project/Blueprints/Triggers/AreaInfo.SelfArea` (`self.SecondArea`)) _asproject_instance)
  (`/Game/Project/Blueprints/Character/Camera.MoveCamera` (`/Game/Project/Blueprints/ProjectInstance.GameCamera` _asproject_instance) (`/Game/Project/Blueprints/Triggers/AreaInfo.CameraPos` (`self.SecondArea`))))

(fn `UserConstructionScript`
  (bind _collidersize (`self.ColliderSize`))
  (`BoxComponent.SetBoxExtent` (`self.Collider`) _collidersize true)
  (`SceneComponent.SetWorldScale3D` (`self.Barrier`) (`KismetMathLibrary.MakeVector` (.x (/ _collidersize 50.0)) 0.0 (.z (/ _collidersize 50.0)))))