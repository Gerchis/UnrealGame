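; CameraLevel is a camera-control Blueprint that turns horizontal and vertical look axes into controller yaw and pitch, scaled by a negated sensitivity.
; Vertical look clamps control rotation pitch to min and max limits, handling the 0–360 wrap by splitting at 180 degrees.
; Within an offset of either limit, a fade factor linearly reduces pitch sensitivity for movement toward that limit, easing the camera into the stop.
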(event `LookHorizontal`
  (params (Axis :type "Float (double-precision)"))
  ;[1 1 1] Camera Horizontal Rotation
  (`self.AddControllerYawInput` (* Axis -1.0 (`self.Sensibility`))))

(event `LookVertical`
  (params (Axis :type "Float (double-precision)"))
  (bind (_returnvalue_roll _returnvalue_pitch) (`KismetMathLibrary.BreakRotator` (`self.GetControlRotation`)))
  (bind (_returnvalue_roll_2 _returnvalue_pitch_2 _returnvalue_yaw) (`KismetMathLibrary.BreakRotator` (`self.GetControlRotation`)))
  (bind (_returnvalue_roll_3 _returnvalue_pitch_3) (`KismetMathLibrary.BreakRotator` (`self.GetControlRotation`)))
  (bind (_returnvalue_roll_4 _returnvalue_pitch_4) (`KismetMathLibrary.BreakRotator` (`self.GetControlRotation`)))
  ;[1 1 1] Camera Vertical Rotation With Limit
  (`self.AddControllerPitchInput` (* Axis -1.0 (`self.Sensibility`) (`self.SensibilityFade`)))
  (if (and (< _returnvalue_pitch (- 360.0 (`self.MaxRotationLimit`))) (< (`self.MinRotationLimit`) _returnvalue_pitch))
    (if (> _returnvalue_pitch_2 180.0)
      (`Controller.SetControlRotation` (`self.GetController`) (`KismetMathLibrary.MakeRotator` _returnvalue_roll_2 (- 360.0 (`self.MaxRotationLimit`)) _returnvalue_yaw))
      (else
        (`Controller.SetControlRotation` (`self.GetController`) (`KismetMathLibrary.MakeRotator` _returnvalue_roll_2 (`self.MinRotationLimit`) _returnvalue_yaw))))
    (else
      ;[1 1 1] FadeToLimit
      (if (or (< (`KismetMathLibrary.Abs` (- (- 360.0 (`self.MaxRotationLimit`)) _returnvalue_pitch_4)) (`self.DistanceFadeOffset`)) (< (`KismetMathLibrary.Abs` (- _returnvalue_pitch_4 (`self.MinRotationLimit`))) (`self.DistanceFadeOffset`)))
        (if (and (> 0.0 Axis) (> _returnvalue_pitch_3 180.0))
          (set `self.SensibilityFade` (/ (`KismetMathLibrary.Abs` (- (- 360.0 (`self.MaxRotationLimit`)) _returnvalue_pitch_3)) (`self.DistanceFadeOffset`)))
          (elif (and (< _returnvalue_pitch_3 180.0) (< 0.0 Axis))
            (set `self.SensibilityFade` (/ (`KismetMathLibrary.Abs` (- _returnvalue_pitch_3 (`self.MinRotationLimit`))) (`self.DistanceFadeOffset`)))
            (else
              (set `self.SensibilityFade` 1.0))))
        (else
          (set `self.SensibilityFade` 1.0))))))

(fn `UserConstructionScript`)