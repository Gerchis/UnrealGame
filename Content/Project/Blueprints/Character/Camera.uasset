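; Player-controlled orbit camera actor that registers itself as GameCamera in ProjectInstance so other code can reach it.
; Turn input yaws the root, LookUp pitches the spring arm within limits, and Zoom changes the clamped arm length.
; Pitch and zoom sensitivity fade as they approach their limits, easing the camera into each stop.
; MoveCamera glides the actor to a new position with a timeline lerp, then stores that position for the next move.
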(event `self.ReceiveBeginPlay`
  (`self.EnableInput` (`GameplayStatics.GetPlayerController` 0))
  (`SceneComponent.K2_AddLocalRotation` (`self.SpringArm`) (`KismetMathLibrary.MakeRotator` 0.0 (* (`self.InitRotation`) -1.0)) false false)
  (set `self.CurrentPos` (`self.K2_GetActorLocation`))
  (set `/Game/Project/Blueprints/ProjectInstance.GameCamera` self (cast `/Game/Project/Blueprints/ProjectInstance` (`GameplayStatics.GetGameInstance`) :!pure true)))

(event `InputAxis|Turn`
  (params (AxisValue :type "Float (single-precision)"))
  ;[1 1 1] HorizontalMovement
  (`SceneComponent.K2_AddWorldRotation` (`self.DefaultSceneRoot`) (`KismetMathLibrary.MakeRotator` 0.0 0.0 (* AxisValue 1.0 (`self.Sensibility`))) false false))

(event `InputAxis|LookUp`
  (params (AxisValue :type "Float (single-precision)"))
  (bind _returnvalue (* AxisValue -1.0))
  (bind (_returnvalue_roll _returnvalue_pitch) (`KismetMathLibrary.BreakRotator` (`SceneComponent.K2_GetComponentRotation` (`self.SpringArm`))))
  (bind (_returnvalue_roll_2 _returnvalue_pitch_2) (`KismetMathLibrary.BreakRotator` (`SceneComponent.K2_GetComponentRotation` (`self.SpringArm`))))
  (bind (_returnvalue_roll_3 _returnvalue_pitch_3 _returnvalue_yaw) (`KismetMathLibrary.BreakRotator` (`SceneComponent.K2_GetComponentRotation` (`self.SpringArm`))))
  (bind (_returnvalue_roll_4 _returnvalue_pitch_4) (`KismetMathLibrary.BreakRotator` (`SceneComponent.K2_GetComponentRotation` (`self.SpringArm`))))
  ;[1 1 1] Camera Vertical Rotation With Limit
  (`SceneComponent.K2_AddLocalRotation` (`self.SpringArm`) (`KismetMathLibrary.MakeRotator` 0.0 (* AxisValue 1.0 (`self.Sensibility`) (`self.SensibilityFade`))) false false)
  (if (not (and (> _returnvalue_pitch_2 (* (`self.MaxRotationLimit`) -1.0)) (> (`self.MinRotationLimit`) _returnvalue_pitch_2)))
    (if (> 0.0 _returnvalue_pitch_3)
      (`SceneComponent.K2_SetWorldRotation` (`self.SpringArm`) (`KismetMathLibrary.MakeRotator` _returnvalue_roll_3 (* (`self.MaxRotationLimit`) -1.0) _returnvalue_yaw) false false)
      (else
        (`SceneComponent.K2_SetWorldRotation` (`self.SpringArm`) (`KismetMathLibrary.MakeRotator` _returnvalue_roll_3 (`self.MinRotationLimit`) _returnvalue_yaw) false false)))
    (else
      ;[1 1 1] FadeToLimit
      (if (or (< (`KismetMathLibrary.Abs` (- (* (`self.MaxRotationLimit`) -1.0) _returnvalue_pitch_4)) (`self.DistanceFadeOffset`)) (< (`KismetMathLibrary.Abs` (- _returnvalue_pitch_4 (`self.MinRotationLimit`))) (`self.DistanceFadeOffset`)))
        (if (and (> _returnvalue 0.0) (> 0.0 _returnvalue_pitch))
          (set `self.SensibilityFade` (/ (`KismetMathLibrary.Abs` (- (* (`self.MaxRotationLimit`) -1.0) _returnvalue_pitch)) (`self.DistanceFadeOffset`)))
          (elif (and (< 0.0 _returnvalue_pitch) (< _returnvalue 0.0))
            (set `self.SensibilityFade` (/ (`KismetMathLibrary.Abs` (- _returnvalue_pitch (`self.MinRotationLimit`))) (`self.DistanceFadeOffset`)))
            (else
              (set `self.SensibilityFade` 1.0))))
        (else
          (set `self.SensibilityFade` 1.0))))))

(event `InputAxis|Zoom`
  (params (AxisValue :type "Float (single-precision)"))
  (bind _returnvalue (+ (* AxisValue (`self.ZoomSensibility`) (`self.ZoomSensibilityFactor`)) (`self.ArmLength`)))
  ;[1 1 1] Zoom
  (if (> _returnvalue (`self.MaxArmLenght`))
    (set `self.ArmLength` (`self.MaxArmLenght`))
    (elif (< _returnvalue (`self.MinArmLenght`))
      (set `self.ArmLength` (`self.MinArmLenght`))
      (else
        (set `self.ArmLength` _returnvalue))))
  (set `SpringArmComponent.TargetArmLength` (`self.ArmLength`) (`self.SpringArm`))
  (if (< (`KismetMathLibrary.Abs` (- (`self.ArmLength`) (`self.MaxArmLenght`))) (`self.ArmDistanceFade`))
    (if (> AxisValue 0.0)
      (set `self.ZoomSensibilityFactor` (/ (`KismetMathLibrary.Abs` (- (`self.ArmLength`) (`self.MaxArmLenght`))) (`self.ArmDistanceFade`)))
      (else
        (set `self.ZoomSensibilityFactor` 1.0 :!label _label)))
    (elif (< (`KismetMathLibrary.Abs` (- (`self.ArmLength`) (`self.MinArmLenght`))) (`self.ArmDistanceFade`))
      (if (< AxisValue 0.0)
        (set `self.ZoomSensibilityFactor` (/ (`KismetMathLibrary.Abs` (- (`self.ArmLength`) (`self.MinArmLenght`))) (`self.ArmDistanceFade`)))
        (else
          (goto _label)))
      (else
        (goto _label)))))

(event `MoveCamera`
  (params (NewPos :type "Vector Structure"))
  (bind (_direction _alpha) (`Timeline|Movement` :!via `PlayFromStart`)
    (:`Update`
      (`self.K2_SetActorLocation` (`KismetMathLibrary.VLerp` (`self.CurrentPos`) NewPos _alpha)))
    (:`Finished`
      (set `self.CurrentPos` (`self.K2_GetActorLocation`)))))

(fn `UserConstructionScript`
  (set `SpringArmComponent.TargetArmLength` (`self.ArmLength`) (`self.SpringArm`)))